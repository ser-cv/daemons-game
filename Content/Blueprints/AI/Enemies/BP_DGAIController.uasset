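; BP_DGAIController is an enemy AI controller that feeds perceived targets into the Blackboard.
; Perception updates store the actor as AimActor, writing it to the Blackboard only when successfully sensed.
; A looping one-second timer copies that actor's position to the AimLocation key.
; The reference is never cleared, so location updates continue after sensing is lost while the actor stays valid.
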(event `self.ReceiveBeginPlay`
  (`KismetSystemLibrary.K2_SetTimerDelegate` (delegate `Update location`) 1.0 true))

(event `self.ReceiveTick`
  (params (DeltaSeconds :type "Float (single-precision)")))

(event `Update location`
  (bind _aimactor (`self.AimActor`))
  (if (`KismetSystemLibrary.IsValid` _aimactor)
    (`BlackboardComponent.SetValueAsVector` (`AIBlueprintHelperLibrary.GetBlackboard` null) "AimLocation" (`self.K2_GetActorLocation` _aimactor))))

(event `self.AIPerception.OnTargetPerceptionUpdated`
  (params (Actor :type "Actor Object Reference") (Stimulus :type "AIStimulus Structure"))
  (`/Engine/EditorBlueprintResources/StandardMacros.IsValid` Actor
    (:`Is Valid`
      (set `self.AimActor` Actor)
      (if (`.bSuccessfullySensed` (break `AIStimulus` Stimulus))
        (`BlackboardComponent.SetValueAsObject` (`AIBlueprintHelperLibrary.GetBlackboard` null) "AimActor" (`self.AimActor`))))))

(fn `UserConstructionScript`)