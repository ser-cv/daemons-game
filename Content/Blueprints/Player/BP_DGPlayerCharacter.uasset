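; Player character Blueprint that provides a cooldown-gated Dash event.
; Dash plays a timeline that feeds CalculateDashForce into CharacterMovement's AddForce on each update, then clears the cooldown after a delay once finished.
; CalculateDashForce contains horizontal force math along the velocity direction, halved off the ground, but that expression is left unused.
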(event `self.Dash`
  (bind _dashspeed (`self.DashSpeed`))
  (bind (_returnvalue_x _returnvalue_y) (`KismetMathLibrary.BreakVector` (`KismetMathLibrary.Normal` (`self.GetVelocity`))))
  (bind (_returnvalue_x_2 _returnvalue_y_2) (`KismetMathLibrary.BreakVector` (`KismetMathLibrary.Normal` (`self.GetVelocity`))))
  (bind _returnvalue (/ (`self.DashSpeed`) 2.0))
  (if (not (`self.bDashCooldown`))
    (set `self.bDashCooldown` true)
    (`Timeline|Timeline` :!via `PlayFromStart`
      (:`Update`
        (`CharacterMovementComponent.AddForce` (`self.CharacterMovement`) (select `bool` (`NavMovementComponent.IsMovingOnGround` (`self.CharacterMovement`)) :`false` (`KismetMathLibrary.MakeVector` (* _returnvalue_x_2 _returnvalue) (* _returnvalue_y_2 _returnvalue)) :`true` (`KismetMathLibrary.MakeVector` (* _returnvalue_x _dashspeed) (* _returnvalue_y _dashspeed)))))
      (:`Finished`
        (`KismetSystemLibrary.Delay` (`self.DashCooldownTime`))
        (set `self.bDashCooldown` false)))))

(fn `UserConstructionScript`)