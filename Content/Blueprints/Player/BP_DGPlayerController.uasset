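; Player controller that lets the player swap between human and mech forms with the E key.
; It checks the current pawn's class, spawns the other character at that pawn's transform, destroys the old pawn and possesses the new one.
; The mech spawns raised above the human's position, and both spawns ignore collision.
; Detach-from-controller nodes remain in the graph but never run.
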(event `Key|E`
  (params (Key :type "Key Structure"))
  (bind _returnvalue (`GameplayStatics.GetPlayerPawn` 0))
  (bind _returnvalue_2 (`self.GetTransform` _returnvalue))
  (:`Pressed`
    (cast `/Game/Blueprints/Player/BP_DGHumanCharacter` _returnvalue
      (:`then`
        (bind _returnvalue_3 (`|SpawnActorFromClass` "/Game/Blueprints/Player/BP_DGMechCharacter.BP_DGMechCharacter_C" (`KismetMathLibrary.MakeTransform` (+ (.location _returnvalue_2) (0.0 0.0 150.0)) (.rotation _returnvalue_2) (.scale _returnvalue_2)) "AlwaysSpawn" "MultiplyWithRoot" null null))
        (`self.K2_DestroyActor` _returnvalue)
        (`self.Possess` _returnvalue_3))
      (:`CastFailed`
        (cast `/Game/Blueprints/Player/BP_DGMechCharacter` _returnvalue)
        (bind _returnvalue_4 (`|SpawnActorFromClass` "/Game/Blueprints/Player/BP_DGHumanCharacter.BP_DGHumanCharacter_C" _returnvalue_2 "AlwaysSpawn" "MultiplyWithRoot" null null))
        (`self.K2_DestroyActor` _returnvalue)
        (`self.Possess` _returnvalue_4)))))

(fn `UserConstructionScript`)