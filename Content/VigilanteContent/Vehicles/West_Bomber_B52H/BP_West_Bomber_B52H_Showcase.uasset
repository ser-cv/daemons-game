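; Showcase variant of the West B-52H bomber Blueprint that exposes the aircraft's adjustable parts through generic checkbox, slider and twin-slider events.
; Each event forwards its value to named setters for damage display, turbines, control surfaces, bomb hatches, light emissivity and landing gear.
; Paired parts mostly share one value, while the twin sliders split front gear from rear and wing gear, and left aileron from right.
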(event `/Game/VigilanteContent/Shared/Blueprints/Showcase/Interfaces/BP_ShowcaseControlsInterface.SetCheckboxVariable0`
  (params (NewState :type Boolean))
  (`self.SetShowDamaged` NewState))

(event `/Game/VigilanteContent/Shared/Blueprints/Showcase/Interfaces/BP_ShowcaseControlsInterface.SetSliderVariable0`
  (params (NewValue :type "Float (single-precision)"))
  (`self.SetTurbineSpeed` NewValue))

(event `/Game/VigilanteContent/Shared/Blueprints/Showcase/Interfaces/BP_ShowcaseControlsInterface.SetSliderVariable1`
  (params (NewValue :type "Float (single-precision)"))
  (`self.SetRudder` NewValue))

(event `/Game/VigilanteContent/Shared/Blueprints/Showcase/Interfaces/BP_ShowcaseControlsInterface.SetSliderVariable2`
  (params (NewValue :type "Float (single-precision)"))
  (`self.SetBombHatchL` NewValue)
  (`self.SetBombHatchR` NewValue))

(event `/Game/VigilanteContent/Shared/Blueprints/Showcase/Interfaces/BP_ShowcaseControlsInterface.SetSliderVariable3`
  (params (NewValue :type "Float (single-precision)"))
  (`self.SetFlapsInnerL` NewValue)
  (`self.SetFlapsInnerR` NewValue))

(event `/Game/VigilanteContent/Shared/Blueprints/Showcase/Interfaces/BP_ShowcaseControlsInterface.SetSliderVariable4`
  (params (NewValue :type "Float (single-precision)"))
  (`self.SetFlapsOuterL` NewValue)
  (`self.SetFlapsOuterR` NewValue))

(event `/Game/VigilanteContent/Shared/Blueprints/Showcase/Interfaces/BP_ShowcaseControlsInterface.SetSliderVariable5`
  (params (NewValue :type "Float (single-precision)"))
  (`self.SetStabilizersL` NewValue)
  (`self.SetStabilizersR` NewValue))

(event `/Game/VigilanteContent/Shared/Blueprints/Showcase/Interfaces/BP_ShowcaseControlsInterface.SetSliderVariable6`
  (params (NewValue :type "Float (single-precision)"))
  (`self.SetLightsEmissivity` NewValue))

(event `/Game/VigilanteContent/Shared/Blueprints/Showcase/Interfaces/BP_ShowcaseControlsInterface.SetTwinSliderVariable0`
  (params (`bFirstSlider?` :type Boolean) (NewFirstValue :type "Float (single-precision)") (NewSecondValue :type "Float (single-precision)"))
  (`self.RetractFrontWheelL` NewFirstValue)
  (`self.RetractFrontWheelR` NewFirstValue)
  (`self.RetractRearRWheel` NewSecondValue)
  (`self.RetractRearLWheel` NewSecondValue)
  (`self.RetractWingLWheel` NewSecondValue)
  (`self.RetractWingRWheel` NewSecondValue))

(event `/Game/VigilanteContent/Shared/Blueprints/Showcase/Interfaces/BP_ShowcaseControlsInterface.SetTwinSliderVariable1`
  (params (`bFirstSlider?` :type Boolean) (NewFirstValue :type "Float (single-precision)") (NewSecondValue :type "Float (single-precision)"))
  (`self.SetAileronL` NewFirstValue)
  (`self.SetAileronR` NewSecondValue))

(fn `UserConstructionScript`
  (`parent.UserConstructionScript`))